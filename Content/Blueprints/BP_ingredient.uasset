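; BP_ingredient is a grabbable pizza ingredient that returns to its starting transform after being used or dropped.
; The Foodtypes value selects its mesh at construction, with meshes set only for pepperoni and cheese.
; Pickup disables physics and attaches it to the given component; Drop re-enables physics, detaches, then resets position after a delay.
; Used resets it immediately; its per-type branches, DropIngredient and the disconnected spawn-copy logic do nothing.
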(event `self.ReceiveBeginPlay`
  (set `self.Starting point` (`self.GetTransform`)))

(event `/Game/VirtualRealityBP/Blueprints/PickupActorInterface.Pickup`
  (params (AttachTo :type "SceneComponent Object Reference"))
  (`PrimitiveComponent.SetSimulatePhysics` (`self.StaticMesh`) false)
  (`SceneComponent.K2_AttachToComponent` (`self.K2_GetRootComponent`) AttachTo "None" "KeepWorld" "KeepWorld" "KeepWorld" false))

(event `Used`
  (switch `/Game/Blueprints/Enum_Food_Types` (`self.Foodtypes`)
    (:`NewEnumerator0`
      _)
    (:`NewEnumerator1`
      _)
    (:`NewEnumerator2`
      _)
    (:`NewEnumerator3`
      _))
  (`self.K2_SetActorTransform` (`self.Starting point`))
  (`PrimitiveComponent.SetSimulatePhysics` (`self.StaticMesh`) false))

(event `/Game/VirtualRealityBP/Blueprints/PickupActorInterface.Drop`
  (`PrimitiveComponent.SetSimulatePhysics` (`self.StaticMesh`) true)
  (`self.K2_DetachFromActor` "KeepWorld" "KeepWorld" "KeepWorld")
  (`KismetSystemLibrary.Delay` 5.0)
  (`self.K2_SetActorTransform` (`self.Starting point`)))

(fn `DropIngredient`
  (returns (NewParam :type "/Game/VirtualRealityBP/Blueprints/BP_IngredientActor Object Reference"))
  (return null))

(fn `UserConstructionScript`
  (`StaticMeshComponent.SetStaticMesh` (`self.StaticMesh`) (select `/Game/Blueprints/Enum_Food_Types` (`self.Foodtypes`) :`NewEnumerator0` "/Game/Blueprints/cylinder.cylinder" :`NewEnumerator1` "/Game/Geometry/Meshes/1M_Cube.1M_Cube" :!type "StaticMesh Object Reference")))