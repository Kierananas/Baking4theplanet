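; Oven actor that cooks Pizza_base actors while they overlap its box trigger.
; Begin overlap tracks the pizza and starts Cooking, a while loop with no delay that calls UpdatePizzaColour on each tracked pizza.
; End overlap removes the pizza and sets IsInOven from a Length < 0 test, which is always false.
; CookingTimes and UpdateMaterial set sphere materials by time or state but are not called here.
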(event `self.ReceiveBeginPlay`)

(event `self.ReceiveActorBeginOverlap`
  (params (OtherActor :type "Actor Object Reference")))

(event `self.Box.OnComponentBeginOverlap`
  (params (OverlappedComponent :type "PrimitiveComponent Object Reference") (OtherActor :type "Actor Object Reference") (OtherComp :type "PrimitiveComponent Object Reference") (OtherBodyIndex :type Integer) (bFromSweep :type Boolean) (SweepResult :type "HitResult Structure (by ref)"))
  (bind _aspizza_base (cast `/Game/Blueprints/Pizza_base` OtherActor))
  (set `self.CurrentPizza` _aspizza_base)
  (`KismetArrayLibrary.Array_AddUnique` (`self.PizzasInOven`) (`self.CurrentPizza`))
  (set `self.bIsInOven` true)
  (`self.Cooking`))

(event `Cooking`
  (while (`self.bIsInOven`)
    (set `self.Cooking time` (`GameplayStatics.GetWorldDeltaSeconds`))
    (for _array_element (`self.PizzasInOven`)
      (`/Game/Blueprints/Pizza_base.UpdatePizzaColour` _array_element)))
  (set `self.Cooking time` 0.0))

(event `self.Box.OnComponentEndOverlap`
  (params (OverlappedComponent :type "PrimitiveComponent Object Reference") (OtherActor :type "Actor Object Reference") (OtherComp :type "PrimitiveComponent Object Reference") (OtherBodyIndex :type Integer))
  (bind _aspizza_base (cast `/Game/Blueprints/Pizza_base` OtherActor))
  (`KismetArrayLibrary.Array_Remove` (`self.PizzasInOven`) (`KismetArrayLibrary.Array_Find` (`self.PizzasInOven`) _aspizza_base))
  (set `self.bIsInOven` (< (`KismetArrayLibrary.Array_Length` (`self.PizzasInOven`)) 0)))

(fn `CookingTimes`
  (bind _sphere (`/Game/Blueprints/Pizza_base.Sphere` (`self.CurrentPizza`)))
  (if (<= (`self.Cooking time`) 15.0) :!label _label
    (`PrimitiveComponent.SetMaterial` _sphere 0 null)
    (elif (<= (`self.Cooking time`) 30.0)
      (`PrimitiveComponent.SetMaterial` _sphere 0 null)
      (elif (<= (`self.Cooking time`) 40.0)
        (`PrimitiveComponent.SetMaterial` _sphere 0 null)
        (else
          (goto _label))))))

(fn `UpdateMaterial`
  (bind _sphere (`/Game/Blueprints/Pizza_base.Sphere` (`self.CurrentPizza`)))
  (switch `/Game/Blueprints/CookingStates` (`self.CookingState`)
    (:`NewEnumerator0`
      (`PrimitiveComponent.SetMaterial` _sphere 0 null))
    (:`NewEnumerator1`
      (`PrimitiveComponent.SetMaterial` _sphere 0 null))
    (:`NewEnumerator2`
      (`PrimitiveComponent.SetMaterial` _sphere 0 null))))

(fn `UserConstructionScript`)