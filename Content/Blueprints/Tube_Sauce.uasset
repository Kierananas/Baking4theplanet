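; Grabbable sauce tube actor that fires sauce projectiles while held.
; Pickup disables mesh physics, sets the grabbed flag, attaches the root to the supplied component and immediately calls SpawnSauce, which spawns Projectile_Sauce at the Shootpoint location only while grabbed.
; Drop clears the flag and detaches the actor but leaves physics simulation off.
; DropIngredient is an empty stub.
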(event `/Game/VirtualRealityBP/Blueprints/PickupActorInterface.Pickup`
  (params (AttachTo :type "SceneComponent Object Reference"))
  (`PrimitiveComponent.SetSimulatePhysics` (`self.StaticMesh`) false)
  (set `self.Isgrabbed` true)
  (`SceneComponent.K2_AttachToComponent` (`self.K2_GetRootComponent`) AttachTo "None" "KeepWorld" "KeepWorld" "KeepWorld" false)
  (`self.spawn sauce`))

(event `spawn sauce`
  (if (`self.Isgrabbed`)
    (`|SpawnActorFromClass` "/Game/Blueprints/Projectile_Sauce.Projectile_Sauce_C" (`KismetMathLibrary.MakeTransform` (`SceneComponent.K2_GetComponentLocation` (`self.Shootpoint`))) "Undefined" "OverrideRootScale" null null)))

(event `/Game/VirtualRealityBP/Blueprints/PickupActorInterface.Drop`
  (set `self.Isgrabbed` false)
  (`PrimitiveComponent.SetSimulatePhysics` (`self.StaticMesh`) false)
  (`self.K2_DetachFromActor` "KeepRelative"))

(fn `DropIngredient`
  (returns (NewParam :type "/Game/VirtualRealityBP/Blueprints/BP_IngredientActor Object Reference"))
  (return null))

(fn `UserConstructionScript`)