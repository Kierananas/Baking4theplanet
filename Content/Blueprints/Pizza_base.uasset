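; Pizza base actor that can be picked up, dropped, topped with ingredients and cooked.
; Overlapping ingredients reveal the matching topping mesh and are used up; overlapping an oven tracks whether the base is inside.
; Pickup attaches the base without physics; dropping detaches it and restores physics only outside an oven.
; UpdatePizzaColour flags cooking and runs a timeline that drives the dynamic material's colour parameter.
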(event `self.ReceiveBeginPlay`
  (bind _returnvalue (`PrimitiveComponent.CreateDynamicMaterialInstance` (`self.Sphere`) 0 null "None"))
  (set `self.Mat_ref` _returnvalue))

(event `/Game/VirtualRealityBP/Blueprints/PickupActorInterface.Pickup`
  (params (AttachTo :type "SceneComponent Object Reference"))
  (`PrimitiveComponent.SetSimulatePhysics` (`self.Sphere`) false :!label _label)
  (`SceneComponent.K2_AttachToComponent` (`self.K2_GetRootComponent`) AttachTo "None" "KeepWorld" "KeepWorld" "KeepWorld" false)
  (if (and false (stale `UpdatePizzaColour` _output_get))
    (goto _label)))

(event `UpdatePizzaColour`
  (set `self.bIsCooking` true)
  (bind (_direction _colour) (`Timeline|Timeline_0` :`NewTime` 40.0 :!via `PlayFromStart`)
    (:`Update`
      _)
    (:`Finished`
      (bind _output_get (set `self.bIsCooking` false))
      (set `self.CookedTime` 0.0)))
  (`MaterialInstanceDynamic.SetVectorParameterValue` (`self.Mat_ref`) "Colour" _colour)
  (bind _output_get_2 (set `self.CookedTime` (`GameplayStatics.GetWorldDeltaSeconds`)))
  (`KismetSystemLibrary.PrintString` (`KismetStringLibrary.Conv_DoubleToString` _output_get_2)))

(event `/Game/VirtualRealityBP/Blueprints/PickupActorInterface.Drop`
  (`self.K2_DetachFromActor` "KeepWorld" "KeepWorld" "KeepWorld")
  (`PrimitiveComponent.SetSimulatePhysics` (`self.Sphere`) (not (`self.bInOven`))))

(event `self.Detect.OnComponentBeginOverlap`
  (params (OverlappedComponent :type "PrimitiveComponent Object Reference") (OtherActor :type "Actor Object Reference") (OtherComp :type "PrimitiveComponent Object Reference") (OtherBodyIndex :type Integer) (bFromSweep :type Boolean) (SweepResult :type "HitResult Structure (by ref)"))
  (bind _asbp_ingredient (cast `/Game/Blueprints/BP_ingredient` OtherActor)
    (:`then`
      (`|ExecutionSequence`
        (:`then_0`
          (switch `/Game/Blueprints/Enum_Food_Types` (`/Game/Blueprints/BP_ingredient.Foodtypes` _asbp_ingredient)
            (:`NewEnumerator0`
              (`SceneComponent.SetVisibility` (`self.Pepperoni`) true false))
            (:`NewEnumerator1`
              (`SceneComponent.SetVisibility` (`self.Cheese`) true false))
            (:`NewEnumerator2`
              (`SceneComponent.SetVisibility` (`self.Mushrooms`) true false))
            (:`NewEnumerator3`
              (`SceneComponent.SetVisibility` (`self.Sauce`) true false))))
        (:`then_1`
          (`/Game/Blueprints/BP_ingredient.Used` _asbp_ingredient))))
    (:`CastFailed`
      (bind _asoven_actor (cast `/Game/Blueprints/Oven_actor` OtherActor))
      (set `self.Oven` _asoven_actor)
      (set `self.bInOven` true))))

(event `self.Detect.OnComponentEndOverlap`
  (params (OverlappedComponent :type "PrimitiveComponent Object Reference") (OtherActor :type "Actor Object Reference") (OtherComp :type "PrimitiveComponent Object Reference") (OtherBodyIndex :type Integer))
  (bind _asoven_actor (cast `/Game/Blueprints/Oven_actor` OtherActor))
  (set `self.Oven` _asoven_actor)
  (set `self.bInOven` false))

(fn `DropIngredient`
  (returns (NewParam :type "/Game/VirtualRealityBP/Blueprints/BP_IngredientActor Object Reference"))
  (return null))

(fn `UserConstructionScript`)