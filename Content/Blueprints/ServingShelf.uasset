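; Serving shelf actor that scores pizzas when they overlap its Box and keeps a running player score.
; BeginPlay creates a Score widget without adding it to the viewport; each Pizza_base overlap adds PizzaScoreFunction's result and updates the widget text.
; PizzaScoreFunction picks points from CookedTime bands, favoring the middle one.
; Its return node is never reached, and times beyond the last band loop back endlessly.
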(event `self.ReceiveBeginPlay`
  (set `self.PlayerScore` 0)
  (bind _returnvalue (`|CreateWidget` "/Game/VirtualRealityBP/Blueprints/Score.Score_C" null (`KismetStringLibrary.Conv_IntToString` (stale `self.Box.OnComponentBeginOverlap` _output_get))))
  (set `self.Score widget` _returnvalue))

(event `self.Box.OnComponentBeginOverlap`
  (params (OverlappedComponent :type "PrimitiveComponent Object Reference") (OtherActor :type "Actor Object Reference") (OtherComp :type "PrimitiveComponent Object Reference") (OtherBodyIndex :type Integer) (bFromSweep :type Boolean) (SweepResult :type "HitResult Structure (by ref)"))
  (bind _aspizza_base (cast `/Game/Blueprints/Pizza_base` OtherActor))
  (bind _playerscore (`self.PizzaScoreFunction` (`/Game/Blueprints/Pizza_base.CookedTime` _aspizza_base)))
  (bind _output_get (set `self.PlayerScore` (+ (`self.PlayerScore`) _playerscore)))
  (set `/Game/VirtualRealityBP/Blueprints/Score.Score` (`KismetStringLibrary.Conv_IntToString` _output_get) (`self.Score widget`)))

(fn `PizzaScoreFunction`
  (params (CookedTime :type "Float (double-precision)"))
  (returns (PlayerScore :type Integer))
  (locals (PizzaScore :type Integer))
  (if (<= CookedTime 15.0) :!label _label
    (set `local.PizzaScore` 50)
    (elif (<= CookedTime 30.0)
      (set `local.PizzaScore` 150)
      (elif (<= CookedTime 40.0)
        (set `local.PizzaScore` 0)
        (else
          (goto _label))))))

(fn `UserConstructionScript`)